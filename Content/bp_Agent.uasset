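; bp_Agent is an unfinished agent actor that appears to prototype flocking-style movement, with Perception and Attraction overlap components.
; Its draft logic moves it along Direction by Speed from the Cone's location, then sums and prints the Direction of overlapping agents.
; None of this runs: Tick is empty, the movement and debug chains are disconnected, and Test returns a zero vector.
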(event EventTick
  (params (DeltaSeconds :type Float%20%28single-precision%29)))

(fn ConstructionScript)

(fn Test
  (params (NewParam :type Rotator))
  (return "0, 0, 0"))

(fn GetDirection
  (params (AgentRef :type Bp%20Agent%20Object%20Reference))
  (return (Variables|bp_Agent_C|GetDirection AgentRef)))