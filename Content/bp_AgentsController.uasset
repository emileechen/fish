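; Controller actor for a fish agent test, spawning a NumFish by NumFish set of Bp_FishAgent actors at BeginPlay and keeping them in an array.
; It sets body length on the first fish only, from twice its mesh bounds radius.
; Pressing W moves only the fish at index 2 as a debug step.
; The shuffled move-all loop and the randomized grid transform in InitLocations are left unconnected.
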(event Custom|debug
  (Default|MoveFish (Utilities|Array|Get(acopy) (Variables|Default|GetfishAgents) 2)))

(event EventBeginPlay
  (bind _numfish (Variables|Default|GetnumFish))
  (bind _returnvalue (- _numfish 1))
  (for _index (range 0 _returnvalue)
    (for _index_2 (range 0 _returnvalue)
      (Utilities|Array|Add (Variables|Default|GetfishIndices) (+ (* _index 10) _index_2))
      (bind _returnvalue_2 (Game|SpawnActorfromClass "/Game/bp_FishAgent.bp_FishAgent_C" (|initlocations _index _index_2) "AlwaysSpawn" 0 0))
      (Utilities|Array|Add (Variables|Default|GetfishAgents) _returnvalue_2)))
  (Input|EnableInput (Game|GetPlayerController 0))
  (|SetBodyLength))

(event EventTick
  (params (DeltaSeconds :type Float%20%28single-precision%29)))

(event Input|KeyboardEvents|W
  (params (Key :type Key%20Structure :default "AnyKey"))
  (:Pressed
    (CallFunction|Debug)))

(fn ConstructionScript)