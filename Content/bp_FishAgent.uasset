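; Fish agent Blueprint that moves in relation to nearby fish, apparently for schooling behavior.
; MoveFish sizes the PerceptionBounds sphere to the computed cohesion radius, then queries overlapping WorldStatic fish agents and passes them to Swim.
; As apparent debug visualization, it tints those neighbors red and then itself green through a material color parameter.
; Tick and construction are empty, so nothing here calls MoveFish.
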(event EventTick
  (params (DeltaSeconds :type Float%20%28single-precision%29)))

(fn ConstructionScript)

(fn MoveFish
  (bind _perceptionbounds (Variables|Default|GetperceptionBounds))
  (bind _returnvalue (Class|FishAgent|CalcCohesionRadius))
  (Components|Sphere|SetSphereRadius _perceptionbounds _returnvalue true)
  (bind _outactors (Class|KismetSystemLibrary|ComponentOverlapActorsNEW _perceptionbounds (Math|Transform|MakeTransform (Transformation|GetActorLocation)) (Utilities|Array|MakeArray "ObjectTypeQuery1") "bp_FishAgent_C"))
  (Class|FishAgent|Swim _outactors)
  (for _array_element _outactors
    (bind _asbp_fish_agent (Utilities|Casting|CastTobp_FishAgent _array_element)
      (:then
        (Rendering|Material|SetVectorParameterValueonMaterials (Actor|GetComponentbyClass _asbp_fish_agent "/Script/Engine.StaticMeshComponent") "color" "1.000000,0.000000, 0"))
      (:CastFailed
        (Development|PrintString "cast fail"))))
  (Rendering|Material|SetVectorParameterValueonMaterials (Actor|GetComponentbyClass "/Script/Engine.StaticMeshComponent") "color" "0.000000,1.000000, 0"))